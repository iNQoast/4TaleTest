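; BP_BaseWeapon is a base skeletal-mesh weapon component for BP_ThirdPersonCharacter, configured from a WeaponInfo struct through UpdateInfo.
; Shortly after BeginPlay it async-loads the weapon mesh and attaches itself to the owner's WeaponSocket.
; For projectile weapons, StartFire fires and starts a looping fire-rate timer that CancelFire clears.
; Each shot plays a montage on the owner and delegates projectile spawning to it from the Muzzle socket.
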(event Custom|SpawnProjectile
  (bind _owner (Variables|Default|GetOwner)
    (:then
      (Default|SpawnProjectile _owner (Transformation|GetSocketLocation "Muzzle") (Variables|Default|GetDamage)))
    (:else)))

(event Custom|WeaponAttach
  (bind _object (Utilities|AsyncLoadAsset (.WeaponMesh (Utilities|Struct|BreakF_WeaponInfo (Variables|Default|GetWeaponInfo))))
    (:Completed
      (bind _asskeletal_mesh (Utilities|Casting|CastToSkeletalMesh _object))
      (Components|SkinnedMesh|SetSkinnedAssetandUpdate _asskeletal_mesh true)
      (Transformation|AttachComponentToComponent (Variables|/Script/Engine.Character|GetMesh (Variables|Default|GetOwner)) "WeaponSocket" "KeepRelative" "KeepRelative" "KeepRelative" true))))

(event Custom|FireProjectile
  (bind _owner (Variables|Default|GetOwner)
    (:then
      (bind _returnvalue (Utilities|LoadAssetBlocking (Utilities|Struct|BreakF_WeaponInfo (Variables|Default|GetWeaponInfo))))
      (bind _asanim_montage (Utilities|Casting|CastToAnimMontage _returnvalue))
      (Animation|PlayAnimMontage _owner _asanim_montage 1.0 "None")
      (CallFunction|SpawnProjectile))
    (:else)))

(event EventBeginPlay
  (bind _asbp_third_person_character (Utilities|Casting|CastToBP_ThirdPersonCharacter (Components|GetOwner)))
  (Variables|Default|SetOwner _asbp_third_person_character)
  (Utilities|FlowControl|Delay 0.2)
  (CallFunction|WeaponAttach))

(event EventTick
  (params (DeltaSeconds :type Float%20%28single-precision%29)))

(event EventStartFire
  (switch Utilities|FlowControl|Switch|SwitchonE_WeaponType (Variables|Default|GetFire%20Type)
    (:NewEnumerator0
      (if (not (Utilities|Time|IsValidTimerHandle (Variables|Default|GetFireTimer)))
        (bind _returnvalue (Utilities|Time|SetTimerbyEvent (EventDispatchers|CreateEvent :!event Custom|FireProjectile) (.FireRate (Utilities|Struct|BreakF_WeaponInfo (Variables|Default|GetWeaponInfo))) true))
        (Variables|Default|SetFireTimer _returnvalue)
        (CallFunction|FireProjectile)))))

(event EventCancelFire
  (Utilities|Time|ClearandInvalidateTimerbyHandle (Variables|Default|GetFireTimer)))

(fn SetName
  (params (Weapon :type Name :default "None")))

(fn UpdateInfo
  (params (WeaponInfo :type F%20Weapon%20Info%20Structure))
  (Variables|Default|SetWeaponInfo WeaponInfo)
  (Variables|Default|SetFire%20Type (.FireType (Utilities|Struct|BreakF_WeaponInfo (Variables|Default|GetWeaponInfo))))
  (Variables|Default|SetDamage (.Damage (Utilities|Struct|BreakF_WeaponInfo (Variables|Default|GetWeaponInfo))))
  (Variables|Default|SetAmmo (.Ammo (Utilities|Struct|BreakF_WeaponInfo (Variables|Default|GetWeaponInfo))))
  (Variables|Default|SetAmmo%20Overall (.AmmoOverall (Utilities|Struct|BreakF_WeaponInfo (Variables|Default|GetWeaponInfo)))))