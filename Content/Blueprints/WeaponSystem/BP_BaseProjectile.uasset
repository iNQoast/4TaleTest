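; BP_BaseProjectile is a weapon projectile that spawns a small explosion emitter wherever it hits.
; Hitting a non-Player actor simply destroys it.
; On a Player-tagged hit other than player 0's pawn, it sends BaseDamage and the hit result to player 0's pawn, not the hit actor, then destroys itself.
; Hits on player 0's own pawn deal no damage and leave the projectile alive.
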(event Collision|EventHit
  (params (MyComp :type Primitive%20Component%20Object%20Reference) (Other :type Actor%20Object%20Reference) (OtherComp :type Primitive%20Component%20Object%20Reference) (bSelfMoved :type Boolean) (HitLocation :type Vector :default "0, 0, 0") (HitNormal :type Vector :default "0, 0, 0") (NormalImpulse :type Vector :default "0, 0, 0") (Hit :type Hit%20Result%20Structure%20%28by%20ref%29))
  (bind _returnvalue (Game|GetPlayerController 0))
  (bind _returnvalue_2 (Pawn|GetControlledPawn _returnvalue))
  (Effects|SpawnEmitteratLocation "/Game/AssetPackage/FXVarietyPack/Particles/P_ky_explosion.P_ky_explosion" HitLocation "0, 0, 0" "0.040000,0.040000,0.040000")
  (if (Actor|ActorHasTag Other "Player")
    (if (!= (.HitActor (Collision|BreakHitResult Hit)) _returnvalue_2)
      (Class|IDamage|SendDamage(Message) _returnvalue_2 (Variables|Default|GetBase%20Damage) Hit)
      (Actor|DestroyActor))
    (else
      (Actor|DestroyActor))))

(fn ConstructionScript)