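; BPC_PlayerStats is an actor component that tracks the health of the third-person player character.
; On BeginPlay it caches its owner as BP_ThirdPersonCharacter.
; DecreaseLife subtracts damage from Health, clamped between zero and one hundred, and at zero calls the owner's CallOnDeath with the damage causer.
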(event EventBeginPlay
  (bind _asbp_third_person_character (Utilities|Casting|CastToBP_ThirdPersonCharacter (Components|GetOwner)))
  (Variables|Default|SetAs%20BP%20Third%20Person%20Character _asbp_third_person_character))

(event EventTick
  (params (DeltaSeconds :type Float%20%28single-precision%29)))

(fn DecreaseLife
  (params (Damage :type Float%20%28double-precision%29) (DamageCauser :type Actor%20Object%20Reference))
  (Variables|Default|SetHealth (Math|Float|Clamp(Float) (- (Variables|Default|GetHealth) Damage) 0.0 1e+02))
  (if (not (> (Variables|Default|GetHealth) 0.0))
    (Default|CallOnDeath (Variables|Default|GetAs%20BP%20Third%20Person%20Character) DamageCauser)))