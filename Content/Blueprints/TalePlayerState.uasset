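; Player state Blueprint that tracks each player's name, number and frag count.
; On non-server instances, BeginPlay waits briefly, then sets the player name from the PlayerId.
; A custom event increments the frag count.
; The Player Number RepNotify calls the player-count-updated dispatcher or function whenever the value replicates.
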(event Custom|FragCountIncr
  (Math|Integer|IncrementInt (Variables|Default|GetFragCount)))

(event EventBeginPlay
  (if (not (Networking|IsServer))
    (Utilities|FlowControl|Delay 1.0)
    (Variables|Default|SetPlayerName (Utilities|String|StringToName (Utilities|String|ToString(Integer) (Variables|Default|GetPlayerId))))))

(fn ConstructionScript)

(fn OnRepPlayerNumber
  (Default|CallOnPlayerCountUpdated))