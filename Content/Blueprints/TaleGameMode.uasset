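; TaleGameMode is a game mode that registers joining players and runs a timed round.
; PostLogin counts each TalePlayerController and stores it in PCList.
; Shortly after BeginPlay, StartGame sets a one-shot RoundEnd timer from RoundTimer and a looping timer that decrements CurrentTime every second.
; RoundEnd only clears the countdown, with game-end logic left as a placeholder, and SetRoundTimer sets the round length.
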(event Custom|DecreaseTimer
  (Variables|Default|SetCurrentTime (- (Variables|Default|GetCurrentTime) 1.0)))

(event Custom|RoundEnd
  ;[1 1 1 1 12] GameEndHere
  (Utilities|Time|ClearandInvalidateTimerbyHandle (Variables|Default|GetT_Round)))

(event EventBeginPlay
  (Utilities|FlowControl|Delay 0.2)
  (CallFunction|StartGame))

(event EventTick
  (params (DeltaSeconds :type Float%20%28single-precision%29)))

(event EventStartGame
  (Utilities|Time|SetTimerbyEvent (delegate Custom|RoundEnd) (Variables|Default|GetRoundTimer))
  (Variables|Default|SetCurrentTime (Variables|Default|GetRoundTimer))
  (bind _returnvalue (Utilities|Time|SetTimerbyEvent (delegate Custom|DecreaseTimer) 1.0 true))
  (Variables|Default|SetT_Round _returnvalue))

(event EventPostLogin
  (params (NewPlayer :type Player%20Controller%20Object%20Reference))
  (bind _astale_player_controller (Utilities|Casting|CastToTalePlayerController NewPlayer))
  (Math|Integer|IncrementInt (Variables|Default|GetPlayerNumber)
    (:%20%20
      (Utilities|Array|AddUnique (Variables|Default|GetPCList) _astale_player_controller))))

(fn ConstructionScript)

(fn SetRoundTimer
  (params (Seconds :type Float%20%28double-precision%29))
  (Variables|Default|SetRoundTimer Seconds))